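; BP_PanCamera is an actor that pans left and right with the mouse, limited to a maximum angle around its starting facing.
; BeginPlay stores the initial yaw as the base.
; Each Tick adds player 0's horizontal mouse delta, scaled by sensitivity, to a clamped pan offset.
; It then sets the actor's yaw to base plus offset, keeping pitch and roll unchanged.
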(event EventBeginPlay
  (Variables|Default|SetBaseYaw (.yaw (Transformation|GetActorRotation))))

(event EventTick
  (params (DeltaSeconds :type Float%20%28single-precision%29))
  (bind _returnvalue (Transformation|GetActorRotation))
  (bind _maxpanangle (Variables|Default|GetMaxPanAngle))
  (bind _output_get (Variables|Default|SetCurrentPan (Math|Float|Clamp(Float) (+ (* (.DeltaX (Class|PlayerController|GetInputMouseDelta (Game|GetPlayerController 0))) (Variables|Default|GetSensitivity)) (Variables|Default|GetCurrentPan)) (* _maxpanangle -1.0) _maxpanangle)))
  (Transformation|SetActorRotation (Math|Rotator|MakeRotator (.roll _returnvalue) (.pitch _returnvalue) (+ _output_get (Variables|Default|GetBaseYaw)))))

(fn ConstructionScript)