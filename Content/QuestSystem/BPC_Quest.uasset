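; Quest component that tracks elimination objectives in the active quest.
; DestroyActors removes the passed actor from the target list of each incomplete elimination objective.
; When a list empties, it marks that objective completed through a by-ref struct write and prints "Quest Completed!", without checking the remaining objectives.
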(event Custom|Destroy%20Actors
  (params (Item%20Retrieved :type Actor%20Object%20Reference))
  (for _array_element (.objectives (Variables|Default|GetActiveQuest))
    (if (and (not (.Completed (Utilities|Struct|BreakS_QuestObjective _array_element))) (.IsActortoEliminate (Utilities|Struct|BreakS_QuestObjective _array_element)))
      (if (> (Utilities|Array|Length (.ActorstoEliminate (Utilities|Struct|BreakS_QuestObjective _array_element))) 0)
        (Utilities|Array|RemoveItem (.ActorstoEliminate (Utilities|Struct|BreakS_QuestObjective _array_element)) Item%20Retrieved)
        (if (== (Utilities|Array|Length (.ActorstoEliminate (Utilities|Struct|BreakS_QuestObjective _array_element))) 0)
          (|SetBy-RefVar _array_element (Utilities|Struct|MakeS_QuestObjective (.Name (Utilities|Struct|BreakS_QuestObjective _array_element)) true 0 false))
          (Development|PrintString "Quest Completed!"))))))