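; Equipment component for BP_ThirdPersonCharacter that lets the player pick up BP_Item actors and store their data.
; On BeginPlay it caches the character's follow and first-person cameras.
; The interact input sphere-traces forward from the first-person camera, or the follow camera if active, against WorldStatic objects with debug drawing.
; A hit BP_Item has its ItemData appended to ItemSlots through AddItem, then is destroyed.
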(event Input|EnhancedActionEvents|EnhancedInputActionIA_Interact
  (params (ActionValue :type Boolean) (ElapsedSeconds :type Float%20%28double-precision%29) (TriggeredSeconds :type Float%20%28double-precision%29) (InputAction :type Input%20Action%20Object%20Reference :default "/Game/Input/Actions/IA_Interact.IA_Interact"))
  (bind _follow_camera (Variables|Default|GetFollow%20Camera))
  (bind _first_person_camera (Variables|Default|GetFirst%20Person%20Camera))
  (bind _returnvalue (Transformation|GetWorldLocation _follow_camera))
  (bind _returnvalue_2 (Transformation|GetWorldLocation _first_person_camera))
  ;[0.15 0.15 0.15 0.5] [E] to Interact
  (:Started
    ;[0.15 0.15 0.15 0.5] allows input for both camera modes
    (if (Components|Activation|IsActive (Variables|Default|GetFollow%20Camera))
      ;[0.15 0.15 0.15 0.5] pick up trace (third person view)
      (bind (_outhit _returnvalue_3) (Collision|SphereTraceForObjects _returnvalue (+ _returnvalue (* (Math|Vector|GetForwardVector (Transformation|GetWorldRotation _follow_camera)) 2.5e+03)) 15.0 (Utilities|Array|MakeArray "ObjectTypeQuery1") false 0 "ForDuration"))
      (if _returnvalue_3
        (bind _asbp_item (Utilities|Casting|CastToBP_Item (.HitActor (Collision|BreakHitResult _outhit))))
        (Development|PrintString "cast success!")
        (CallFunction|AddItem (Variables|/Game/QuestSystem/InventorySystem/BP_Item.BP_Item_C|GetItemData _asbp_item))
        (Actor|DestroyActor _asbp_item)
        (Development|PrintString "Item Picked Up")
        (else
          (Development|PrintString "Hit fail")))
      (else
        ;[0.15 0.15 0.15 0.5] pick up trace (first person view)
        (bind (_outhit_2 _returnvalue_4) (Collision|SphereTraceForObjects _returnvalue_2 (+ _returnvalue_2 (* (Math|Vector|GetForwardVector (Transformation|GetWorldRotation _first_person_camera)) 2.5e+03)) 15.0 (Utilities|Array|MakeArray "ObjectTypeQuery1") false 0 "ForDuration"))
        (if _returnvalue_4
          (bind _asbp_item_2 (Utilities|Casting|CastToBP_Item (.HitActor (Collision|BreakHitResult _outhit_2))))
          (Development|PrintString "cast success!")
          (CallFunction|AddItem (Variables|/Game/QuestSystem/InventorySystem/BP_Item.BP_Item_C|GetItemData _asbp_item_2))
          (Actor|DestroyActor _asbp_item_2)
          (Development|PrintString "Item Picked Up")
          (else
            (Development|PrintString "Hit fail")))))))

(event EventBeginPlay
  (bind _asbp_third_person_character (Utilities|Casting|CastToBP_ThirdPersonCharacter (Components|GetOwner)))
  (Variables|Default|SetFollow%20Camera (Variables|/Game/ThirdPerson/Blueprints/BP_ThirdPersonCharacter.BP_ThirdPersonCharacter_C|GetFollowCamera _asbp_third_person_character))
  (Variables|Default|SetFirst%20Person%20Camera (Variables|/Game/ThirdPerson/Blueprints/BP_ThirdPersonCharacter.BP_ThirdPersonCharacter_C|GetFirstPersonCamera _asbp_third_person_character)))

(fn AddItem
  (params (NewItem :type S%20Slots%20Structure%20%28by%20ref%29))
  (Utilities|Array|Add (Variables|Default|GetItemSlots) NewItem))