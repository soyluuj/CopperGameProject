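; Quest component that tracks one active quest, its collection objectives and its completion state, and drives the Quest_HUD widget it creates on BeginPlay.
; CollectItem removes the item from a working copy of an unfinished objective's ActorsToEliminate list, writes it back by reference and completes the objective when empty.
; Once all objectives are complete, it clears the quest, sets a completion flag and plays the HUD animation and sound.
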(event Custom|Set%20Active%20Quest%20Text
  (Rendering|Components|TextRender|SetText (Variables|/Game/QuestSystem/Quest_HUD.Quest_HUD_C|GetActiveQuestText (Variables|Default|GetQuest%20HUD%20Widget)) (Utilities|Text|ToText(String) (.QuestName (Utilities|Struct|BreakS_Quest (Variables|Default|GetActive%20Quest)))))
  (Default|ShowQuestPanel (Variables|Default|GetQuest%20HUD%20Widget)))

(event Custom|Set%20Objectives
  (Default|FillObjectives (Variables|Default|GetQuest%20HUD%20Widget) (.objectives (Variables|Default|GetActive%20Quest))))

(event Custom|Collect%20Item
  (params (Item%20Collected :type Actor%20Object%20Reference))
  (for _array_element (.objectives (Variables|Default|GetActive%20Quest))
    (if (and (not (.Completed (Utilities|Struct|BreakS_QuestObjective _array_element))) (.IsActortoEliminate (Utilities|Struct|BreakS_QuestObjective _array_element)))
      (if (!= (Utilities|Array|Length (Variables|Default|GetItemActorArray)) 0)
        _
        (else
          (bind _output_get (Variables|Default|SetItemActorArray (.ActorstoEliminate (Utilities|Struct|BreakS_QuestObjective _array_element))))))
      (Utilities|Array|RemoveItem _output_get Item%20Collected)
      (|SetBy-RefVar _array_element (Utilities|Struct|MakeS_QuestObjective (.Name (Utilities|Struct|BreakS_QuestObjective _array_element)) false (Variables|Default|GetItemActorArray) (.IsActortoEliminate (Utilities|Struct|BreakS_QuestObjective _array_element))))
      (Development|PrintString (Utilities|String|ToString(Integer) (Utilities|Array|Length (Variables|Default|GetItemActorArray))))
      (if (== (Utilities|Array|Length (Variables|Default|GetItemActorArray)) 0)
        (|SetBy-RefVar _array_element (Utilities|Struct|MakeS_QuestObjective (.Name (Utilities|Struct|BreakS_QuestObjective _array_element)) true 0 (.IsActortoEliminate (Utilities|Struct|BreakS_QuestObjective _array_element))))
        (Default|CompleteObjective (Variables|Default|GetQuest%20HUD%20Widget) _array_element)
        (CallFunction|QuestCompleted)))))

(event Custom|Quest%20Completed
  (Math|Integer|IncrementInt (Variables|Default|GetObjectives%20Completed)
    (:%20%20
      (if (>= (Variables|Default|GetObjectives%20Completed) (Utilities|Array|Length (.objectives (Variables|Default|GetActive%20Quest))))
        (Variables|Default|SetActive%20Quest "")
        (Variables|Default|SetObjectives%20Completed 0)
        (Variables|Default|SetQuest%20Completed? true)
        (Default|PlayQuestCompletedAnimation (Variables|Default|GetQuest%20HUD%20Widget))
        (Audio|PlaySound2D "/Game/SFX/quest/benkirb-shine-10-268906.benkirb-shine-10-268906" 1.0 1.0 0.0 0 0)))))

(event EventBeginPlay
  (bind _returnvalue (UserInterface|CreateWidget "/Game/QuestSystem/Quest_HUD.Quest_HUD_C"))
  (bind _output_get (Variables|Default|SetQuest%20HUD%20Widget _returnvalue))
  (UserInterface|Viewport|AddtoViewport _output_get 0)
  (Default|HideQuestPanel (Variables|Default|GetQuest%20HUD%20Widget)))

(event EventInteract
  (if (Variables|Default|GetQuest%20Completed?)
    (Development|PrintString "Quest is Complete")
    (else
      (Development|PrintString "Quest is Incomplete"))))

(fn NewFunction
  (return (Variables|Default|GetQuest%20Completed?)))