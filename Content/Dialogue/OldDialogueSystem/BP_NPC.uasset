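; NPC Blueprint for scripted conversations between Copper and Catrick, in the old dialogue system folder.
; Each Dialogue event advances an index through DialogueScript and updates WB_TestDialogueWidget, choosing name and portrait by whether the index is in CopperLines.
; If the widget is missing, that call only creates and displays it.
; Move and look input are ignored while lines show, then reset when the script ends and the widget is removed.
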(event EventDialogue
  (bind _returnvalue (Game|GetPlayerController 0))
  (bind _returnvalue_2 (Game|GetPlayerController 0))
  ;[0.15 0.15 0.15 0.5] NPC Dialogue System
  ;;[0.15 0.15 0.15 0.5] Dialogue Cycling
  (Math|Integer|IncrementInt (Variables|Default|Getdialogue_index)
    (:%20%20
      (if (< (Variables|Default|Getdialogue_index) (Utilities|Array|Length (Variables|Default|Getdialogue_script)))
        ;;[0.15 0.15 0.15 0.5] Creates the dialogue widget and adds it to the viewport. Along with the dialogue text, character portrait, and character name.
        (Variables|Default|Getcharacter_dialogue
          (:then
            ;;[0.15 0.15 0.15 0.5] Distinguishes which dialogue is from the npc and which is copper's. Sets the character portrait accordingly.
            (if (Utilities|Array|ContainsItem (Variables|Default|Getcopper_lines) (Variables|Default|Getdialogue_index))
              ;;;[0.15 0.3913 0.15 0.5 11] Change the texture for the character portraits and the text for the character names according to needs.
              (Appearance|SetBrushfromTexture (Variables|/Game/Dialogue/OldDialogueSystem/WB_TestDialogueWidget.WB_TestDialogueWidget_C|Getcharacter_portrait (Variables|Default|Getcharacter_portrait)) "/Game/Dialogue/OldDialogueSystem/TestCharacterPortraits/copper.copper" true)
              (Rendering|Components|TextRender|SetText (Variables|/Game/Dialogue/OldDialogueSystem/WB_TestDialogueWidget.WB_TestDialogueWidget_C|Getcharacter_name (Variables|Default|Getcharacter_name)) "Copper")
              (else
                (Appearance|SetBrushfromTexture (Variables|/Game/Dialogue/OldDialogueSystem/WB_TestDialogueWidget.WB_TestDialogueWidget_C|Getcharacter_portrait (Variables|Default|Getcharacter_portrait)) "/Game/Dialogue/OldDialogueSystem/TestCharacterPortraits/catnpc.catnpc" true)
                (Rendering|Components|TextRender|SetText (Variables|/Game/Dialogue/OldDialogueSystem/WB_TestDialogueWidget.WB_TestDialogueWidget_C|Getcharacter_name (Variables|Default|Getcharacter_name)) "Catrick")))
            ;;[0.15 0.15 0.15 0.5] Sets the text to be displayed on the dialogue widget. also while in dialogue, movement is disabled.
            (Rendering|Components|TextRender|SetText (Variables|/Game/Dialogue/OldDialogueSystem/WB_TestDialogueWidget.WB_TestDialogueWidget_C|Getdialogue_text (Variables|Default|Getcharacter_dialogue)) (Utilities|Text|ToText(String) (Utilities|Array|Get(acopy) (Variables|Default|Getdialogue_script) (Variables|Default|Getdialogue_index))))
            (Input|SetIgnoreMoveInput _returnvalue_2 true)
            (Input|SetIgnoreLookInput _returnvalue_2 true))
          (:else
            (bind _returnvalue_3 (UserInterface|CreateWidget "/Game/Dialogue/OldDialogueSystem/WB_TestDialogueWidget.WB_TestDialogueWidget_C" (Game|GetPlayerController 0)))
            (bind _output_get (Variables|Default|Setcharacter_dialogue _returnvalue_3))
            (bind _output_get_2 (Variables|Default|Setcharacter_portrait _output_get))
            (bind _output_get_3 (Variables|Default|Setcharacter_name _output_get_2))
            (UserInterface|Viewport|AddtoViewport _output_get_3 0)))
        (else
          ;;[0.15 0.15 0.15 0.5] When dialogue is finished. Removes the dialogue UI from the screen and enables movement again.
          (Widget|RemovefromParent (Variables|Default|Getcharacter_dialogue))
          (Input|ResetIgnoreMoveInput _returnvalue)
          (Input|ResetIgnoreLookInput _returnvalue))))))

(fn ConstructionScript)