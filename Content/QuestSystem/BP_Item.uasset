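; Collectible quest item that shows an interaction prompt when the player character is nearby.
; While CanInteract is set, entering the Box pops up a UI_Interact widget, outlines the Cube through an overlay material and sets CanPressE.
; Leaving reverses the animation, clears the outline and flag, then removes the widget after a short delay.
; ItemPickedUp passes the item to the player's BPCQuest1 component via CollectItem, then destroys the actor.
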(event OnComponentBeginOverlap(Box)
  (params (OverlappedComponent :type Primitive%20Component%20Object%20Reference) (OtherActor :type Actor%20Object%20Reference) (OtherComp :type Primitive%20Component%20Object%20Reference) (OtherBodyIndex :type Integer) (bFromSweep :type Boolean) (SweepResult :type Hit%20Result%20Structure%20%28by%20ref%29))
  (bind _widget (Variables|Default|GetWidget))
  ;[0.15 0.15 0.15 0.5] UI + Highlight Pop up
  (Utilities|Casting|CastToBP_ThirdPersonCharacter OtherActor)
  (if (Variables|Default|GetCanInteract)
    (bind _returnvalue (UserInterface|CreateWidget "/Game/QuestSystem/UI_Interact.UI_Interact_C"))
    (bind _output_get (Variables|Default|SetInteractionWidget _returnvalue))
    (UserInterface|SetWidget _widget _output_get)
    (Rendering|SetVisibility _widget true false)
    (bind _interactionwidget (Variables|Default|GetInteractionWidget)
      (:then
        (if (not (Variables|Default|GetHintVisible))
          (UserInterface|Animation|PlayAnimation _interactionwidget (Variables|/Game/QuestSystem/UI_Interact.UI_Interact_C|GetPopUp _interactionwidget) 0.0 1 "Forward" 1.5 false)
          (Variables|Default|SetHintVisible true)
          (Rendering|Material|SetOverlayMaterial (Variables|Default|GetCube) "/Game/QuestSystem/M_Outline.M_Outline" :!class /Script/Engine.MeshComponent)
          (Variables|Default|SetCanPressE true)))
      (:else))))

(event OnComponentEndOverlap(Box)
  (params (OverlappedComponent :type Primitive%20Component%20Object%20Reference) (OtherActor :type Actor%20Object%20Reference) (OtherComp :type Primitive%20Component%20Object%20Reference) (OtherBodyIndex :type Integer))
  ;[0.15 0.15 0.15 0.5] UI + Highlight Pop up
  (Utilities|Casting|CastToBP_ThirdPersonCharacter OtherActor)
  (if (Variables|Default|GetCanInteract)
    (bind _interactionwidget (Variables|Default|GetInteractionWidget)
      (:then
        (if (Variables|Default|GetHintVisible)
          (UserInterface|Animation|PlayAnimation _interactionwidget (Variables|/Game/QuestSystem/UI_Interact.UI_Interact_C|GetPopUp _interactionwidget) 0.0 1 "Reverse" 1.5 false)
          (Variables|Default|SetHintVisible false)
          (Variables|Default|SetCanPressE false)
          (Rendering|Material|SetOverlayMaterial (Variables|Default|GetCube) 0 :!class /Script/Engine.MeshComponent))
        (Utilities|FlowControl|Delay 0.15)
        (Widget|RemovefromParent (Variables|Default|GetInteractionWidget))
        (Variables|Default|SetInteractionWidget 0)
        (Rendering|SetVisibility (Variables|Default|GetWidget) false false))
      (:else))))

(event Custom|ItemPickedUp
  (bind _asbp_third_person_character (Utilities|Casting|CastToBP_ThirdPersonCharacter (Game|GetPlayerCharacter 0)))
  (Default|CollectItem (Variables|/Game/ThirdPerson/Blueprints/BP_ThirdPersonCharacter.BP_ThirdPersonCharacter_C|GetBPC_Quest1 _asbp_third_person_character) self)
  (Actor|DestroyActor))

(fn ConstructionScript)