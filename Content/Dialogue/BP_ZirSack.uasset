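; BP_ZirSack is an interactable dialogue Blueprint, apparently for a character named ZirSack, that plays a conversation one line per interaction.
; On Interact, it creates a CatrickDialogue widget if needed, fills in speaker and text from the indexed Dialogue array, and advances the index.
; Player move and look input are ignored until an interaction past the last line removes the widget and restores input.
; The index never resets, so the conversation plays only once.
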(event EventBeginPlay)

(event Collision|EventActorBeginOverlap
  (params (OtherActor :type Actor%20Object%20Reference)))

(event EventTick
  (params (DeltaSeconds :type Float%20%28single-precision%29)))

(event EventInteract
  (bind _returnvalue (Game|GetPlayerController 0))
  (bind _returnvalue_2 (Game|GetPlayerController 0))
  (if (< (Variables|Default|GetDialogueIndex) (Utilities|Array|Length (Variables|Default|GetDialogue)))
    (Variables|Default|Getdialogue_text
      (:then
        _)
      (:else
        (bind _returnvalue_3 (UserInterface|CreateWidget "/Game/Dialogue/CatrickDialogue.CatrickDialogue_C" (Game|GetPlayerController 0)))
        (bind _output_get (Variables|Default|Setdialogue_text _returnvalue_3))
        (bind _output_get_2 (Variables|Default|Setcharacter_name _output_get))
        (UserInterface|Viewport|AddtoViewport _output_get_2 0)))
    (Rendering|Components|TextRender|SetText (Variables|/Game/Dialogue/CatrickDialogue.CatrickDialogue_C|Getcharacter_name (Variables|Default|Getcharacter_name)) (Utilities|Text|ToText(String) (.speakername (Utilities|Array|Get(acopy) (Variables|Default|GetDialogue) (Variables|Default|GetDialogueIndex)))))
    (Rendering|Components|TextRender|SetText (Variables|/Game/Dialogue/CatrickDialogue.CatrickDialogue_C|Getdialogue_text (Variables|Default|Getdialogue_text)) (Utilities|Text|ToText(String) (.lineoftext (Utilities|Array|Get(acopy) (Variables|Default|GetDialogue) (Variables|Default|GetDialogueIndex)))))
    (Math|Integer|IncrementInt (Variables|Default|GetDialogueIndex)
      (:%20%20
        (Input|SetIgnoreMoveInput _returnvalue_2 true)
        (Input|SetIgnoreLookInput _returnvalue_2 true)))
    (else
      (Widget|RemovefromParent (Variables|Default|Getdialogue_text))
      (Input|ResetIgnoreMoveInput _returnvalue)
      (Input|ResetIgnoreLookInput _returnvalue))))

(fn ConstructionScript)